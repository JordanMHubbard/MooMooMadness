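; Game mode for Destroy It All, a timed multiplayer match in which players control cows and the highest score wins.
; PostLogin registers each controller, shows its lobby, and spawns and possesses a BP_Cow at an index-named player start.
; A one-shot countdown unfreezes players and starts a looping timer that decrements the time stored in the game state.
; When time expires it freezes everyone, shows each player the outcome, then ends sessions after a delay.
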(event `StartMatchTimer`
  (set `/Game/Blueprints/GS_DestroyItAll.CurrentTime` (`self.MatchTime`) (`self.GS_DIA`))
  (`self.ShowTimers`)
  (bind _returnvalue (`KismetSystemLibrary.K2_SetTimerDelegate` (delegate `UpdateMatchTimer`) 1.0 true))
  (set `self.MatchTimerHandle` _returnvalue))

(event `self.ReceiveBeginPlay`
  (bind _asgs_destroy_it_all (cast `/Game/Blueprints/GS_DestroyItAll` (`GameplayStatics.GetGameState`)))
  (set `self.GS_DIA` _asgs_destroy_it_all))

(event `UpdateMatchTimer`
  (if (> (`/Game/Blueprints/GS_DestroyItAll.CurrentTime` (`self.GS_DIA`)) 0)
    (`/Engine/EditorBlueprintResources/StandardMacros.DecrementInt` (`/Game/Blueprints/GS_DestroyItAll.CurrentTime` (`self.GS_DIA`)))
    (else
      (`KismetSystemLibrary.K2_PauseTimerHandle` (`self.MatchTimerHandle`))
      (`self.FreezeAll`)
      (`self.CalculateWinner`)
      (`KismetSystemLibrary.Delay` 4.0)
      (for _array_element (`self.PlayerControllers`)
        (`/Game/Blueprints/PC_DestroyItAll.EndSession` _array_element)))))

(event `self.K2_PostLogin`
  (params (NewPlayer :type "PlayerController Object Reference"))
  (bind _playercontrollers (`self.PlayerControllers`))
  (bind _aspc_destroy_it_all (cast `/Game/Blueprints/PC_DestroyItAll` NewPlayer))
  (`KismetArrayLibrary.Array_Add` (`self.PlayerControllers`) _aspc_destroy_it_all)
  (`self.InitializeController` _aspc_destroy_it_all)
  (bind _returnvalue (`|SpawnActorFromClass` "/Game/ThirdPerson/Blueprints/BP_Cow.BP_Cow_C" (`self.GetTransform` (`self.K2_FindPlayerStart` NewPlayer (`KismetStringLibrary.Conv_IntToString` (- (`KismetArrayLibrary.Array_Length` (`self.PlayerControllers`)) 1)))) "Undefined" "MultiplyWithRoot" null null))
  (`Controller.Possess` NewPlayer _returnvalue)
  (for _array_element _playercontrollers
    (`/Game/Blueprints/PC_DestroyItAll.UpdatePlayerCount` _array_element (`KismetArrayLibrary.Array_Length` _playercontrollers))))

(event `ShowTimers`
  (for _array_element (`self.PlayerControllers`)
    (`/Game/Blueprints/PC_DestroyItAll.ShowMatchTimer` _array_element)))

(event `RemoveMatchLobbies`
  (for _array_element (`self.PlayerControllers`)
    (`/Game/Blueprints/PC_DestroyItAll.RemoveMatchLobby` _array_element)))

(event `StartCountdown`
  (`/Engine/EditorBlueprintResources/StandardMacros.DoOnce` false
    (:`Completed`
      (for _array_element (`self.PlayerControllers`)
        (`/Game/Blueprints/PC_DestroyItAll.ShowCountdown` _array_element))
      (`KismetSystemLibrary.Delay` 5.0)
      (`self.UnfreezeAll`)
      (`self.StartMatchTimer`))))

(event `UnfreezeAll`
  (for _array_element (`self.PlayerControllers`)
    (`/Game/Blueprints/PC_DestroyItAll.Unfreeze` _array_element)))

(event `FreezeAll`
  (for _array_element (`self.PlayerControllers`)
    (`/Game/Blueprints/PC_DestroyItAll.ShowTimesUp` _array_element)
    (`/Game/Blueprints/PC_DestroyItAll.Freeze` _array_element)))

(fn `CalculateWinner`
  (bind _outactors (`GameplayStatics.GetAllActorsOfClass` "/Game/ThirdPerson/Blueprints/BP_Cow.BP_Cow_C"))
  (for _array_element _outactors
    (bind _score (`MooMooMadnessCharacter.Score` _array_element))
    (if (> _score (`self.HighestScore`))
      (set `self.HighestScore` _score)
      (set `self.WinningCow` _array_element)))
  (for _array_element_2 (`self.PlayerControllers`)
    (`/Game/Blueprints/PC_DestroyItAll.ShowMatchOutcome` _array_element_2 (== _array_element_2 (`Pawn.GetController` (`self.WinningCow`)))))
  (return))

(fn `InitializeController`
  (params (Controller :type "/Game/Blueprints/PC_DestroyItAll Object Reference"))
  (`/Game/Blueprints/PC_DestroyItAll.ShowMatchLobby` Controller)
  (return))

(fn `UserConstructionScript`)