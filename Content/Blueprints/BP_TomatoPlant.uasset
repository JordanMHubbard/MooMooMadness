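; BP_TomatoPlant is a tomato plant actor with randomized looks and a destruction sound.
; Its construction script gives the static mesh a random, slightly enlarged uniform scale and the actor a random yaw, so placed plants vary.
; A PlaySound event plays the plant destruction cue at the actor's location; nothing in this Blueprint calls it or destroys the plant.
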(event `self.PlaySound`
  (`GameplayStatics.PlaySoundAtLocation` "/Game/Sounds/SC_PlantDestruction.SC_PlantDestruction" (`self.K2_GetActorLocation`) (struct) 1.0 1.0 0.0 null null null null))

(fn `UserConstructionScript`
  (`SceneComponent.SetWorldScale3D` (`self.StaticMesh`) (* (`KismetMathLibrary.MakeVector` 1.0 1.0 1.0) (/ (`KismetMathLibrary.Conv_IntToDouble` (`KismetMathLibrary.RandomIntegerInRange` 110 140)) 100.0)))
  (`self.K2_SetActorRotation` (`KismetMathLibrary.MakeRotator` 0.0 0.0 (`KismetMathLibrary.Conv_IntToDouble` (`KismetMathLibrary.RandomIntegerInRange` 0 360)))))