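; BP_Destroyable is an actor Blueprint, named as a destroyable prop, that varies its look per instance and provides a destruction sound.
; The construction script gives the static mesh a random uniform world scale, treating MinScale and MaxScale as integer percentages, and the actor a random yaw.
; The PlaySound event plays DestructionSound at the actor's location if valid; the graphs shown contain no destruction logic or caller for it.
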(event `self.PlaySound`
  (bind _destructionsound (`self.DestructionSound`))
  (`/Engine/EditorBlueprintResources/StandardMacros.IsValid` _destructionsound
    (:`Is Valid`
      (`GameplayStatics.PlaySoundAtLocation` _destructionsound (`self.K2_GetActorLocation`) (struct) 1.0 1.0 0.0 null null null null))))

(fn `UserConstructionScript`
  (`SceneComponent.SetWorldScale3D` (`self.StaticMesh`) (* (`KismetMathLibrary.MakeVector` 1.0 1.0 1.0) (/ (`KismetMathLibrary.Conv_IntToDouble` (`KismetMathLibrary.RandomIntegerInRange` (`self.MinScale`) (`self.MaxScale`))) 100.0)))
  (`self.K2_SetActorRotation` (`KismetMathLibrary.MakeRotator` 0.0 0.0 (`KismetMathLibrary.Conv_IntToDouble` (`KismetMathLibrary.RandomIntegerInRange` 0 360)))))