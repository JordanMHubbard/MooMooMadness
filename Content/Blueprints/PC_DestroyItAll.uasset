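; Player controller for the multiplayer Destroy It All match, handling each player's UI and input through the match flow.
; Events create the lobby (with a guest mode for non-servers), countdown, match timer and win/lose outcome widgets, and update the lobby's player count.
; Leaving the lobby restores the HUD_Cow UI, while Freeze and Unfreeze toggle pawn input.
; It also fades in music after the countdown appears and leaves sessions via BP_GameInstance.
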(event `ShowCountdown`
  (bind _returnvalue (`|CreateWidget` "/Game/ThirdPerson/UI/WBP_Countdown.WBP_Countdown_C"))
  (bind _output_get (set `self.CountdownWidget` _returnvalue))
  (`UserWidget.AddToViewport` _output_get 0)
  (`KismetSystemLibrary.Delay` 5.0)
  (bind _returnvalue_2 (`AddComponent|NODE_AddAudioComponent-0`))
  (bind _output_get_2 (set `self.BGMusic` _returnvalue_2))
  (`AudioComponent.FadeIn` _output_get_2 2.0 0.2 0.0 "Linear"))

(event `ShowTimesUp`
  (set `TextBlock.Text` "Times Up!" (`/Game/ThirdPerson/UI/WBP_Countdown.Countdown` (`self.CountdownWidget`))))

(event `EndSession`
  (bind _asbp_game_instance (cast `/Game/Blueprints/BP_GameInstance` (`GameplayStatics.GetGameInstance`)))
  (`/Game/Blueprints/BP_GameInstance.LeaveSession` _asbp_game_instance))

(event `ShowMatchTimer`
  (bind _returnvalue (`|CreateWidget` "/Game/ThirdPerson/UI/WBP_MatchTimer.WBP_MatchTimer_C"))
  (`UserWidget.AddToViewport` _returnvalue 0))

(event `ShowMatchLobby`
  (set `self.bShowMouseCursor` true)
  (bind _returnvalue (`|CreateWidget` "/Game/Levels/MainMenu/WBP_StartMatch.WBP_StartMatch_C"))
  (set `self.MatchLobbyWidget` _returnvalue)
  (if (not (`KismetSystemLibrary.IsServer`))
    (`/Game/Levels/MainMenu/WBP_StartMatch.IsGuest` (`self.MatchLobbyWidget`)))
  (`UserWidget.AddToViewport` (`self.MatchLobbyWidget`) 0))

(event `Unfreeze`
  (`self.EnableInput` (`self.K2_GetPawn`) self))

(event `RemoveMatchLobby`
  (set `self.bShowMouseCursor` false)
  (bind _ashud_cow (cast `/Game/Blueprints/HUD_Cow` (`self.GetHUD`)))
  (`UserWidget.AddToViewport` (`/Game/Blueprints/HUD_Cow.UI_Ref` _ashud_cow) 0)
  (`Widget.RemoveFromParent` (`self.MatchLobbyWidget`)))

(event `Freeze`
  (`self.DisableInput` (`self.K2_GetPawn`) self))

(event `UpdatePlayerCount`
  (params (NumPlayers :type Integer))
  (`TextBlock.SetText` (`/Game/Levels/MainMenu/WBP_StartMatch.NumPlayers` (`self.MatchLobbyWidget`)) (`KismetTextLibrary.Conv_IntToText` NumPlayers)))

(event `ShowMatchOutcome`
  (params (IsWinner :type Boolean))
  (`WidgetLayoutLibrary.RemoveAllWidgets`)
  (bind _returnvalue (`|CreateWidget` "/Game/ThirdPerson/UI/WBP_MatchOutcome.WBP_MatchOutcome_C"))
  (if IsWinner
    (`/Game/ThirdPerson/UI/WBP_MatchOutcome.SetWinner` _returnvalue))
  (`UserWidget.AddToViewport` _returnvalue 0))

(fn `UserConstructionScript`)