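; BP_Bush2 is a bush actor that can vary its static mesh for visual variety.
; Its construction script runs the parent's script, then, if IsRandomMesh is set, randomly assigns one of two bush meshes to the StaticMesh component.
; The event graph holds only disabled default event stubs, so it adds no runtime logic of its own.
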(fn `UserConstructionScript`
  (`parent.UserConstructionScript`)
  (if (`self.IsRandomMesh`)
    (`StaticMeshComponent.SetStaticMesh` (`self.StaticMesh`) (select `int` (`KismetMathLibrary.RandomInteger` 2) :`0` (`self.Bush1`) :`1` (`self.Bush2`)))))